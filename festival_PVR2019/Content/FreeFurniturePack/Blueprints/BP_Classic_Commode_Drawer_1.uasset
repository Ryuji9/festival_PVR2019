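; Classic commode drawer actor that slides open and closed when its PointOfViewEvent is triggered.
; A FlipFlop alternates an instant, unswept local offset along the Y axis, out and back, with no animation.
; A refrigerator-open sound is spawned at the actor's location as feedback.
; BeginPlay, overlap and Tick events are disabled stubs, so all behavior runs from that one event.
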(event `self.point of view event`
  (`/Engine/EditorBlueprintResources/StandardMacros.FlipFlop`
    (:`A`
      (`self.K2_AddActorLocalOffset` (0.0 20.0 0.0)))
    (:`B`
      (`self.K2_AddActorLocalOffset` (0.0 -20.0 0.0))))
  (`GameplayStatics.SpawnSoundAtLocation` "/Game/FreeFurniturePack/Blueprints/refrigerator-open1.refrigerator-open1" (`self.K2_GetActorLocation`) (struct) 5.0 1.0 0.0 null null))

(fn `UserConstructionScript`
  (`parent.UserConstructionScript`))