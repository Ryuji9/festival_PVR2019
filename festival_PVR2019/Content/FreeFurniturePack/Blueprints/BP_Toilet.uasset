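; BP_Toilet is a toilet furniture Blueprint that plays a toilet sound at its own location.
; PointOfViewEvent passes through a DoOnce, spawns the Toilet1 sound, then resets the gate after a ten-second delay so repeat triggers are throttled.
; The construction script only calls its parent, and BeginPlay, overlap and Tick are disabled stubs.
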(event `self.point of view event`
  (`/Engine/EditorBlueprintResources/StandardMacros.DoOnce` false :!label _label
    (:`Completed`
      (`GameplayStatics.SpawnSoundAtLocation` "/Game/FreeFurniturePack/Blueprints/toilet1.toilet1" (`self.K2_GetActorLocation`) (struct) 1.0 1.0 0.0 null null)
      (`KismetSystemLibrary.Delay` 10.0)
      (goto _label :!via `Reset`))))

(fn `UserConstructionScript`
  (`parent.UserConstructionScript`))