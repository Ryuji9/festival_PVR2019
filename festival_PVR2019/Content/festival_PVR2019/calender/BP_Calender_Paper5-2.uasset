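; Calendar paper Blueprint that tears away and falls when its PointOfViewEvent fires.
; The event enables physics simulation on the Sphere component, then a DoOnce plays a paper-tear sound at the actor's location.
; After a short delay the actor destroys itself.
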(event `self.point of view event`
  (`PrimitiveComponent.SetSimulatePhysics` (`self.Sphere`) true)
  (`/Engine/EditorBlueprintResources/StandardMacros.DoOnce` false
    (:`Completed`
      (`GameplayStatics.SpawnSoundAtLocation` "/Game/festival_PVR2019/calender/paper-tear3.paper-tear3" (`self.K2_GetActorLocation`) (struct) 1.0 1.0 0.0 null null)
      (`KismetSystemLibrary.Delay` 1.0)
      (`self.K2_DestroyActor`))))

(fn `UserConstructionScript`
  (`parent.UserConstructionScript`))