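; BP_card2 is a solution checker for a rotation puzzle in the festival_PVR2019 project, apparently a card puzzle.
; Every Tick it compares the rotations of ten referenced puzzle actors to hard-coded targets within a one-degree tolerance.
; Most pieces are tested on pitch alone, while Puzzle41, Puzzle42 and Puzzle5 compare the full rotator.
; When all match, it only prints a debug "Hello", repeating each frame while solved.
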(event `self.ReceiveTick`
  (params (DeltaSeconds :type "Float (single-precision)"))
  (bind (_returnvalue_roll _returnvalue_pitch) (`KismetMathLibrary.BreakRotator` (`self.K2_GetActorRotation` (`self.Puzzle2-2`))))
  (bind (_returnvalue_roll_2 _returnvalue_pitch_2) (`KismetMathLibrary.BreakRotator` (`self.K2_GetActorRotation` (`self.Puzzle2-4`))))
  (bind (_returnvalue_roll_3 _returnvalue_pitch_3) (`KismetMathLibrary.BreakRotator` (`self.K2_GetActorRotation` (`self.Puzzle2-1`))))
  (bind (_returnvalue_roll_4 _returnvalue_pitch_4) (`KismetMathLibrary.BreakRotator` (`self.K2_GetActorRotation` (`self.Puzzle2-3`))))
  (bind (_returnvalue_roll_5 _returnvalue_pitch_5) (`KismetMathLibrary.BreakRotator` (`self.K2_GetActorRotation` (`self.Puzzle3-1`))))
  (bind (_returnvalue_roll_6 _returnvalue_pitch_6) (`KismetMathLibrary.BreakRotator` (`self.K2_GetActorRotation` (`self.Puzzle3-2`))))
  (bind (_returnvalue_roll_7 _returnvalue_pitch_7) (`KismetMathLibrary.BreakRotator` (`self.K2_GetActorRotation` (`self.Puzzle6`))))
  (if (and (`KismetMathLibrary.NearlyEqual_FloatFloat` _returnvalue_pitch_3 0.0 1.0) (`KismetMathLibrary.NearlyEqual_FloatFloat` _returnvalue_pitch 0.0 1.0) (`KismetMathLibrary.NearlyEqual_FloatFloat` _returnvalue_pitch_4 0.0 1.0) (`KismetMathLibrary.NearlyEqual_FloatFloat` _returnvalue_pitch_2 0.0 1.0) (`KismetMathLibrary.NearlyEqual_FloatFloat` _returnvalue_pitch_5 90.0 1.0) (`KismetMathLibrary.NearlyEqual_FloatFloat` _returnvalue_pitch_6 90.0 1.0) (== (`self.K2_GetActorRotation` (`self.Puzzle4-1`)) (struct :`Yaw` 180.0 :`Roll` -180.0) :`ErrorTolerance` 1.0) (== (`self.K2_GetActorRotation` (`self.Puzzle4-2`)) (struct :`Yaw` 180.0 :`Roll` -180.0) :`ErrorTolerance` 1.0) (== (`self.K2_GetActorRotation` (`self.Puzzle5`)) (struct) :`ErrorTolerance` 1.0) (`KismetMathLibrary.NearlyEqual_FloatFloat` _returnvalue_pitch_7 -90.0 1.0))
    (`KismetSystemLibrary.PrintString` "Hello")))

(fn `UserConstructionScript`)