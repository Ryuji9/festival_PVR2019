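; BP_Puzzle is a festival PVR2019 puzzle Blueprint that reacts to a point-of-view event.
; When PointOfViewEvent fires, the actor rotates a quarter turn in world space and then calls Puzzle on its Card2 reference.
; Tick and the construction script only call their parents, so all puzzle behavior here is event-driven.
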(event `self.point of view event`
  (`self.K2_AddActorWorldRotation` (struct :`Pitch` -90.0))
  (`/Game/festival_PVR2019/Puzzle/BP_card2.Puzzle` (`self.card2`)))

(event `self.ReceiveTick`
  (params (DeltaSeconds :type "Float (single-precision)"))
  (`parent.ReceiveTick` DeltaSeconds))

(fn `UserConstructionScript`
  (`parent.UserConstructionScript`))