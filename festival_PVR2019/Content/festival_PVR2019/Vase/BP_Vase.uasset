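; Vase actor with a destructible mesh, SMVaseDM, that takes damage when its PointOfViewEvent fires.
; The event calls ApplyDamage at the actor's location with zero impulse strength, so the hit adds no push.
; BeginPlay and the construction script only call the parent, and the overlap and Tick events are disabled.
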(event `self.ReceiveBeginPlay`
  (`parent.ReceiveBeginPlay`))

(event `self.point of view event`
  (bind _returnvalue (`self.K2_GetActorLocation`))
  (`DestructibleComponent.ApplyDamage` (`self.SM_Vase_DM`) 1.0 _returnvalue _returnvalue 0.0))

(fn `UserConstructionScript`
  (`parent.UserConstructionScript`))