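; BP_DoorLock is a door lock display actor that shows text on two TextRender components.
; At BeginPlay it sets TextRender1 to the Abc value.
; Each Tick it shows the first three characters of the Reply string on TextRender and prints the full string on screen for debugging.
; Nothing in this graph writes Reply or performs any locking.
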(event `self.ReceiveBeginPlay`
  (`TextRenderComponent.K2_SetText` (`self.TextRender1`) (`self.abc`)))

(event `self.ReceiveTick`
  (params (DeltaSeconds :type "Float (single-precision)"))
  (`TextRenderComponent.K2_SetText` (`self.TextRender`) (`KismetTextLibrary.Conv_StringToText` (`KismetStringLibrary.Left` (`self.reply`) 3)))
  (`KismetSystemLibrary.PrintString` (`self.reply`) true true (struct :`G` 0.66 :`B` 1.0 :`A` 1.0) DeltaSeconds))

(fn `UserConstructionScript`)