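; BP_Button-3 is the digit 3 button for a door lock.
; When its PointOfViewEvent fires, it prepends "3" to the Reply string on the referenced Doorlock, so entered digits build up in reverse order.
; It contains no other active logic, leaving any checking of the code outside this Blueprint.
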(event `self.point of view event`
  (bind _doorlock (`self.doorlock`))
  (set `/Game/festival_PVR2019/doorlock/BP_DoorLock.reply` (`KismetStringLibrary.Concat_StrStr` "3" (`/Game/festival_PVR2019/doorlock/BP_DoorLock.reply` _doorlock)) _doorlock))

(fn `UserConstructionScript`
  (`parent.UserConstructionScript`))